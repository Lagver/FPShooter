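; StarForge_BP is a progression actor that opens the Star Forge widget when something overlaps its box trigger.
; The widget is created for player 0 on first overlap, cached and reused, and input switches to UI-only with the cursor shown.
; Ending the overlap removes the widget and restores game-only input, in logic marked as temporary.
; Neither event checks which actor triggered the overlap.
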(event `self.Box.OnComponentBeginOverlap`
  (params (OverlappedComponent :type "PrimitiveComponent Object Reference") (OtherActor :type "Actor Object Reference") (OtherComp :type "PrimitiveComponent Object Reference") (OtherBodyIndex :type Integer) (bFromSweep :type Boolean) (SweepResult :type "HitResult Structure (by ref)"))
  (bind _returnvalue (`GameplayStatics.GetPlayerController` 0))
  ;[1 1 1] InIt UI
  (`/Engine/EditorBlueprintResources/StandardMacros.IsValid` (`self.StarForgeWBVar`)
    (:`Is Valid`
      (`UserWidget.AddToViewport` (`self.StarForgeWBVar`) 0))
    (:`Is Not Valid`
      (bind _returnvalue_2 (`|CreateWidget` "/Game/FPShooter/Assets/UI/StarForge/StarForge_WB.StarForge_WB_C" _returnvalue))
      (bind _output_get (set `self.StarForgeWBVar` _returnvalue_2))
      (`UserWidget.AddToViewport` _output_get 0)))
  (`WidgetBlueprintLibrary.SetInputMode_UIOnlyEx` _returnvalue null)
  (set `PlayerController.bShowMouseCursor` true _returnvalue))

(event `self.Box.OnComponentEndOverlap`
  (params (OverlappedComponent :type "PrimitiveComponent Object Reference") (OtherActor :type "Actor Object Reference") (OtherComp :type "PrimitiveComponent Object Reference") (OtherBodyIndex :type Integer))
  (bind _returnvalue (`GameplayStatics.GetPlayerController` 0))
  ;[1 1 1] Временно
  (`Widget.RemoveFromParent` (`self.StarForgeWBVar`))
  (set `PlayerController.bShowMouseCursor` false _returnvalue)
  (`WidgetBlueprintLibrary.SetInputMode_GameOnly` _returnvalue))

(fn `UserConstructionScript`)